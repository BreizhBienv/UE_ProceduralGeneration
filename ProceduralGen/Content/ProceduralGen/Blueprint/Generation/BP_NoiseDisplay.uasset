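; Noise preview actor that shows a generated 2D fractal (fBm) Perlin noise map on a plane.
; The Construction Script scales the plane to the map size, generates noise from the exposed parameters and remaps it from -1..1 to 0..1.
; The values become a texture fed to a dynamic M_Noise material instance.
; A Cellular Automata call is present but unconnected, and the event graph is unused.
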(event EventBeginPlay)

(event Collision|EventActorBeginOverlap
  (params (OtherActor :type Actor%20Object%20Reference)))

(event EventTick
  (params (DeltaSeconds :type Float%20%28single-precision%29)))

(fn ConstructionScript
  (Transformation|SetWorldScale3D (Variables|Default|GetPlane) (Math|Vector|MakeVector (Math|Conversions|ToFloat(Integer) (Variables|Noise|GetMapWidth)) (Math|Conversions|ToFloat(Integer) (Variables|Noise|GetMapHeight)) 1.0))
  (bind _returnvalue (Rendering|Material|CreateDynamicMaterialInstance (Variables|Default|GetPlane) 0 "/Game/ProceduralGen/Ressources/Materials/M_Noise.M_Noise" "None" :!class /Script/Engine.PrimitiveComponent))
  (bind _returnvalue_2 (Class|ProceduralAlgoFunctionLibrary|FbmPerlinNoiseMap2D (Variables|Noise|GetMapWidth) (Variables|Noise|GetMapHeight) (Variables|Noise|GetScale) (Variables|Noise|GetOrigin) (Variables|Noise|FBM|GetOctaves) (Variables|Noise|FBM|GetPercistence) (Variables|Noise|FBM|GetLacunarity)))
  (bind _returnvalue_3 (Class|ProceduralAlgoFunctionLibrary|RemapArray _returnvalue_2 (Math|Vector2D|MakeVector2D -1.0 1.0) (Math|Vector2D|MakeVector2D 0.0 1.0)))
  (bind _returnvalue_4 (Class|ProceduralAlgoFunctionLibrary|Texturefrom2DNoiseMap (Variables|Noise|GetMapWidth) (Variables|Noise|GetMapHeight) _returnvalue_3))
  (Rendering|Material|SetTextureParameterValue _returnvalue "DynamicTexture" _returnvalue_4))