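; BP_NoiseDisplay is an actor that previews a cellular automata noise map on a plane for grid generation.
; Its construction script scales the plane to the map size and builds the map from density, iteration, morph and border settings.
; The map becomes a texture fed into a dynamic M_Noise material, so the preview refreshes whenever construction reruns.
; An fBm Perlin noise alternative is present but disconnected.
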(event EventBeginPlay)

(event Collision|EventActorBeginOverlap
  (params (OtherActor :type Actor%20Object%20Reference)))

(event EventTick
  (params (DeltaSeconds :type Float%20%28single-precision%29)))

(fn ConstructionScript
  (Transformation|SetWorldScale3D (Variables|Default|GetPlane) (Math|Vector|MakeVector (Math|Conversions|ToFloat(Integer) (Variables|Noise|GetMapWidth)) (Math|Conversions|ToFloat(Integer) (Variables|Noise|GetMapHeight)) 1.0))
  (bind _returnvalue (Rendering|Material|CreateDynamicMaterialInstance (Variables|Default|GetPlane) 0 "/Game/GridSystem/Ressources/Materials/M_Noise.M_Noise" "None" :!class /Script/Engine.PrimitiveComponent))
  (bind _returnvalue_2 (Class|ProceduralAlgoFunctionLibrary|CellularAutomata (Variables|Noise|GetMapWidth) (Variables|Noise|GetMapHeight) (Variables|Noise|Automata|GetDensity) (Variables|Noise|Automata|GetIterations) (Variables|Noise|Automata|GetMorph%20Factor) (Variables|Noise|Automata|GetFill%20Border)))
  (bind _returnvalue_3 (Class|ProceduralAlgoFunctionLibrary|Texturefrom2DNoiseMap (Variables|Noise|GetMapWidth) (Variables|Noise|GetMapHeight) _returnvalue_2))
  (Rendering|Material|SetTextureParameterValue _returnvalue "DynamicTexture" _returnvalue_3))